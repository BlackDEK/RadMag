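; BP_Map is the map actor that spawns and tracks the world's BP_Chunk actors.
; Init stores the GameDataManager and executes a MakeSystemChunkCounter request through it, with the map passed in.
; OnGetChunkCounter receives the count and drives SpawnChunk, which spawns chunks at the origin, owned by the map.
; Each chunk joins the Chunks array and is initialized with its array index as Id plus the same manager.
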(event `self.ReceiveBeginPlay`)

(event `self.OnGetChunkCounter`
  (params (ChunkCounter :type Integer))
  (`self.Spawn Chunk` ChunkCounter))

(fn `Get Chunk Counter`
  (bind _returnvalue (`RenderSystems.MakeSystemChunkCounter` self self))
  (`GameDataManager.Execute` (`self.GameDataManager`) _returnvalue)
  (return))

(fn `Init`
  (params (GameDataManager :type "GameDataManager Object Reference"))
  (set `self.GameDataManager` GameDataManager)
  (`self.Get Chunk Counter`)
  (return))

(fn `Spawn Chunk`
  (params (Count :type Integer))
  (for _ (range (+ Count 1))
    (bind _returnvalue (`|SpawnActorFromClass` "/Game/MainLevel/BP_Chunk.BP_Chunk_C" (`KismetMathLibrary.MakeTransform` (0.0 0.0 0.0)) "DontSpawnIfColliding" "OverrideRootScale" self null))
    (bind _returnvalue_2 (`KismetArrayLibrary.Array_Add` (`self.Chunks`) _returnvalue))
    (`/Game/MainLevel/BP_Chunk.Init` _returnvalue _returnvalue_2 (`self.GameDataManager`)))
  (return))

(fn `UserConstructionScript`)