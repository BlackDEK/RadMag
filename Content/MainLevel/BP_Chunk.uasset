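; BP_Chunk is a chunk actor that displays generated geometry as a procedural mesh.
; Init stores an Id and GameDataManager, adds a ProceduralMeshComponent, and has the manager execute a SystemGenerateChunkCache built for this chunk.
; OnCreateChunk turns supplied vertices, triangles and linear vertex colors into a mesh section with collision.
; GetId returns 0 rather than the stored Id.
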(event `self.OnCreateChunk`
  (params (Vertices :type "Array of Vector Structure (by ref)") (Triangles :type "Array of Integer (by ref)") (VertexColors :type "Array of LinearColor Structure (by ref)"))
  (`ProceduralMeshComponent.CreateMeshSection_LinearColor` :`self` (`self.Mesh`) :`Vertices` Vertices :`Triangles` Triangles :`VertexColors` VertexColors :`bCreateCollision` true))

(fn `GetId`
  (returns (ReturnValue :type Integer))
  (return 0))

(fn `Init`
  (params (Id :type Integer) (GameDataManager :type "GameDataManager Object Reference"))
  (set `self.Id` Id)
  (set `self.GameDataManager` GameDataManager)
  (bind _returnvalue (`AddComponent|NODE_AddProceduralMeshComponent-1` :`RelativeTransform` (`KismetMathLibrary.MakeTransform` (0.0 0.0 0.0))))
  (set `self.Mesh` _returnvalue)
  (bind _returnvalue_2 (`RenderSystems.MakeSystemGenerateChunkCache` self self))
  (`GameDataManager.Execute` (`self.GameDataManager`) _returnvalue_2)
  (return))

(fn `UserConstructionScript`)