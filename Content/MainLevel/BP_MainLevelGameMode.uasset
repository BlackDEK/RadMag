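; BP_MainLevelGameMode is the main level's game mode, which bootstraps the world and player when play begins.
; It constructs a GameDataManager object and runs a world-generation system on it, configured by chunk counts and chunk size.
; It then spawns and initializes BP_Map and passes the data manager to the main level player controller's Init.
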(event `self.ReceiveBeginPlay`
  (`self.Create Game Data Manager`)
  (`self.Generate World`)
  (`self.Create Map`)
  (`self.Init Player`))

(fn `Create Game Data Manager`
  (bind _returnvalue (`|GenericCreateObject` "/Script/RadMag.GameDataManager" self))
  (bind _output_get (set `self.GameDataManager` _returnvalue))
  (`GameDataManager.CreateGameData` _output_get)
  (return))

(fn `Create Map`
  (bind _returnvalue (`|SpawnActorFromClass` "/Game/MainLevel/BP_Map.BP_Map_C" (`KismetMathLibrary.MakeTransform` (0.0 0.0 0.0)) "DontSpawnIfColliding" "OverrideRootScale" self null))
  (bind _output_get (set `self.Map` _returnvalue))
  (`/Game/MainLevel/BP_Map.Init` _output_get)
  (return))

(fn `Generate World`
  (locals (ChunkCountOX :type Integer :default 1) (ChunkCountOY :type Integer :default 1) (ChunkSize :type Integer :default 16))
  (bind _returnvalue (`GenerateWorldSystem.MakeSystemGenerateWorld` (make `CreateGameRulesContext` (`local.ChunkCountOX`) (`local.ChunkCountOY`) (`local.ChunkSize`)) (`self.GameDataManager`)))
  (`GameDataManager.Execute` (`self.GameDataManager`) _returnvalue)
  (return))

(fn `Init Player`
  (bind _asbp_main_level_player_controller (cast `/Game/MainLevel/BP_MainLevelPlayerController` (`GameplayStatics.GetPlayerController` 0)))
  (`/Game/MainLevel/BP_MainLevelPlayerController.Init` _asbp_main_level_player_controller (`self.GameDataManager`))
  (return))

(fn `UserConstructionScript`)