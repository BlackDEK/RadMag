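; Player controller for the main level that spawns a top-down BP_Camera pawn on BeginPlay and possesses it.
; Left click traces under the cursor and, when it hits a BP_Chunk, passes the hit location to CallHitResult and prints it for debugging.
; An Init function stores the GameDataManager and hands it to BP_MainLevelHUD for setup.
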(event `self.ReceiveBeginPlay`
  (bind _returnvalue (`|SpawnActorFromClass` "/Game/MainLevel/BP_Camera.BP_Camera_C" (`KismetMathLibrary.MakeTransform` (0.0 0.0 100.0) (struct :`Pitch` -90.0 :`Roll` -90.0)) "DontSpawnIfColliding" "OverrideRootScale" self null))
  (bind _output_get (set `self.MainPawn` _returnvalue))
  (`self.Possess` _output_get))

(event `Key|LeftMouseButton`
  (params (Key :type "Key Structure"))
  (:`Pressed`
    (`self.TouchMap`)))

(fn `CreateHUD`
  (bind _asbp_main_level_hud (cast `/Game/MainLevel/BP_MainLevelHUD` (`self.GetHUD`)))
  (bind _output_get (set `self.HUD` _asbp_main_level_hud))
  (`/Game/MainLevel/BP_MainLevelHUD.Init` _output_get (`self.GameDataManager`))
  (return))

(fn `Init`
  (params (GameDataManager :type "GameDataManager Object Reference"))
  (set `self.GameDataManager` GameDataManager)
  (`self.CreateHUD`)
  (return))

(fn `TouchMap`
  (locals (LocalLocation :type "Vector Structure" :default (0.0 0.0 0.0)))
  (bind (_bblockinghit _binitialoverlap _time _distance _location _impactpoint _normal _impactnormal _physmat _hitactor) (`GameplayStatics.BreakHitResult` (`self.GetHitResultUnderCursorByChannel` "TraceTypeQuery1")))
  (if _bblockinghit
    (if (== (`GameplayStatics.GetObjectClass` _hitactor) "/Game/MainLevel/BP_Chunk.BP_Chunk_C")
      (bind _output_get (set `local.LocalLocation` _location))
      (`self.HitResult` _output_get)
      (`KismetSystemLibrary.PrintString` (`KismetStringLibrary.Conv_VectorToString` _output_get) true true (struct :`R` 0.17946 :`G` 0.221648 :`B` 1.0 :`A` 1.0))
      (return))))

(fn `UserConstructionScript`)